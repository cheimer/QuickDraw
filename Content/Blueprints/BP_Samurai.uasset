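; Samurai character for a draw-timing duel game, with sprite-based idle, attack and defeated states.
; It slides in on begin play and on reset, using timelines to lerp the sprite position.
; An attack during the game mode's Wait phase shows a cross and locks out further input.
; During Draw it ends the game, lunges, swaps sprite mid-timeline and reports success along with whether the samurai is player controlled.
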(event Custom|SlideIn
  (Components|Timeline|SetPlayRate (Variables|Default|GetSlideTimeLine) 2.0)
  (bind _alpha (Timeline|SlideTimeLine PlayFromStart)
    (:Update
      (Transformation|SetRelativeLocation (Variables|Default|GetPaperSprite) (Math|Vector|Lerp(Vector) (Variables|Default|GetSplideStartPos) (Variables|Default|GetSpriteDefaultPos) _alpha) false false))))

(event Custom|Attack
  (if (not (Variables|Default|GetPressedDraw))
    (switch Utilities|FlowControl|Switch|SwitchonE_Phase (Variables|/Game/Blueprints/GameModeBase_Duel.GameModeBase_Duel_C|GetPhase (Variables|Default|GetGameMode))
      (:NewEnumerator1
        (CallFunction|SetCrossVisibility true)
        (Variables|Default|SetPressedDraw true))
      (:NewEnumerator2
        (Variables|Default|SetPressedDraw true)
        (Default|SetGameFinished (Variables|Default|GetGameMode))
        (bind _alpha (Timeline|AttackAnimTimeLine PlayFromStart)
          (:Update
            (Transformation|SetRelativeLocation (Variables|Default|GetPaperSprite) (Math|Vector|Lerp(Vector) (Variables|Default|GetSpriteDefaultPos) (Variables|/Script/Engine.SceneComponent|GetRelativeLocation (Variables|Default|GetAttackPos)) _alpha) false false))
          (:SwitchSprite
            (Rendering|Components|Sprite|SetSprite (Variables|Default|GetPaperSprite) (Variables|Default|GetAttackSprite))
            (Default|AttackedSuccess (Variables|Default|GetGameMode) (Pawn|IsPlayerControlled))))))))

(event Custom|Defeated
  (Rendering|Components|Sprite|SetSprite (Variables|Default|GetPaperSprite) (Variables|Default|GetDefeatedSprite))
  (CallFunction|SetCrossVisibility false))

(event EventBeginPlay
  (bind _asgame_mode_base_duel (Utilities|Casting|CastToGameModeBase_Duel (Game|GetGameMode)))
  (Variables|Default|SetGameMode _asgame_mode_base_duel)
  (Variables|Default|SetSpriteDefaultPos (Variables|/Script/Engine.SceneComponent|GetRelativeLocation (Variables|Default|GetPaperSprite)))
  (CallFunction|Slidein)
  (CallFunction|SetCrossVisibility false))

(fn ConstructionScript)

(fn SetCrossVisibility
  (params (bNewVisibility :type Boolean))
  (Rendering|SetVisibility (Variables|Default|GetCross) bNewVisibility false))

(fn Reset
  (Rendering|Components|Sprite|SetSprite (Variables|Default|GetPaperSprite) (Variables|Default|GetIdleSprite))
  (Variables|Default|SetPressedDraw false)
  (CallFunction|Slidein))